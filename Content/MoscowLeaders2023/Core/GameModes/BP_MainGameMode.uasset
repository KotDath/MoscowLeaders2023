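; Game mode for a timed checkpoint race, running the start countdown, time limit and end-of-race results.
; It binds to every checkpoint's events to handle the finish line and time bonuses, which restart the limit timer with added time.
; A very long timer serves as a stopwatch.
; Finishing or timing out swaps the HUD for the result widget and saves any lower elapsed time as high score, regardless of win.
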(event Custom|Game%20Start
  (bind _returnvalue (Utilities|Time|SetTimerbyEvent (delegate Custom|LoseOutOfTime) (Variables|Default|GetStartRaceTime)))
  (Variables|Default|SetCurrentTime _returnvalue)
  (bind _returnvalue_2 (Utilities|Time|SetTimerbyEvent (delegate Custom|CustomEvent) 1e+09))
  (Variables|Default|SettimeLine _returnvalue_2))

(event Custom|Game%20Finish
  (params (isWin :type Boolean))
  (bind _returnvalue (Game|GetPlayerController 0))
  (Utilities|FlowControl|Sequence
    (:then_0
      (if (> (Variables|Default|GetHighScore) (Class|KismetSystemLibrary|GetTimerElapsedTimeHandle (Variables|Default|GettimeLine)))
        (Variables|Default|SetHighScore (Class|KismetSystemLibrary|GetTimerElapsedTimeHandle (Variables|Default|GettimeLine)))
        (bind _returnvalue_2 (SaveGame|DoesSaveGameExist (Variables|Default|GetslotName)))
        (if _returnvalue_2
          (bind _returnvalue_3 (SaveGame|LoadGamefromSlot (Variables|Default|GetslotName)))
          (bind _output_get (Variables|Default|SetsubclassOfSaver _returnvalue_3))
          (bind _asbp_high_score (Utilities|Casting|CastToBP_HighScore _output_get))
          (Variables|/Game/MoscowLeaders2023/Core/FileSystem/BP_HighScore.BP_HighScore_C|SethighScore _asbp_high_score (Variables|Default|GetHighScore))
          (SaveGame|SaveGametoSlot _asbp_high_score (Variables|Default|GetslotName))
          (else
            (bind _returnvalue_4 (SaveGame|CreateSaveGameObject "/Game/MoscowLeaders2023/Core/FileSystem/BP_HighScore.BP_HighScore_C"))
            (bind _output_get_2 (Variables|Default|SetsubclassOfSaver _returnvalue_4))
            (bind _asbp_high_score_2 (Utilities|Casting|CastToBP_HighScore _output_get_2))
            (Variables|/Game/MoscowLeaders2023/Core/FileSystem/BP_HighScore.BP_HighScore_C|SethighScore _asbp_high_score_2 (Variables|Default|GetHighScore))
            (SaveGame|SaveGametoSlot _asbp_high_score_2 (Variables|Default|GetslotName))))
        (Development|PrintString (Utilities|String|ToString(Float) (Variables|Default|GetHighScore)))))
    (:then_1
      (Variables|/Script/Engine.PlayerController|SetbShowMouseCursor _returnvalue true)
      (bind _asbp_vehicle_player_controller (Utilities|Casting|CastToBP_VehiclePlayerController _returnvalue))
      (Widget|RemovefromParent (Variables|/Game/MoscowLeaders2023/Characters/SportCar/BP_VehiclePlayerController.BP_VehiclePlayerController_C|GetVehicleHud _asbp_vehicle_player_controller)))
    (:then_2
      (bind _returnvalue_5 (UserInterface|CreateWidget "/Game/MoscowLeaders2023/Core/UI/BP_Result.BP_Result_C"))
      (UserInterface|Viewport|AddtoViewport _returnvalue_5 0))
    (:then_3
      (Utilities|Time|PauseTimerbyHandle (Variables|Default|GettimeLine)))))

(event Custom|Start%20Countdown
  (bind _returnvalue (Utilities|Time|SetTimerbyEvent (delegate Custom|CustomEvent_0) (Variables|Default|GetCountdownStartDelay)))
  (Variables|Default|SetcountdownTime _returnvalue)
  (bind _returnvalue_2 (UserInterface|CreateWidget "/Game/MoscowLeaders2023/Core/UI/BP_StartDelay.BP_StartDelay_C"))
  (UserInterface|Viewport|AddtoViewport _returnvalue_2 0))

(event Custom|LoseOutOfTime
  (CallFunction|GameFinish false))

(event Custom|WinCrossTheFinish
  (Utilities|Time|ClearandInvalidateTimerbyHandle (Variables|Default|GetCurrentTime))
  (CallFunction|GameFinish true))

(event Custom|AddTime
  (params (TimeToGive :type Float%20%28double-precision%29))
  (CallFunction|AddTimetoTimer TimeToGive))

(event Custom|CustomEvent)

(event Custom|CustomEvent_0
  (Widget|RemovefromParent (stale Custom|Start%20Countdown _returnvalue_2))
  (Development|PrintString "Let's GOOOO")
  (CallFunction|GameStart))

(event EventBeginPlay
  (Utilities|FlowControl|Sequence
    (:then_0
      (bind _outactors (Actor|GetAllActorsOfClass "/Game/MoscowLeaders2023/Core/Interactables/BP_Checkpoint.BP_Checkpoint_C"))
      (for _array_element _outactors
        (if (Variables|/Game/MoscowLeaders2023/Core/Interactables/BP_Checkpoint.BP_Checkpoint_C|GetisFinishLine _array_element)
          (EventDispatchers|BindEventtoOnCheckpointCross _array_element (EventDispatchers|CreateEvent :!event Custom|WinCrossTheFinish))
          (else
            (EventDispatchers|BindEventtoOnCheckpointTime _array_element (EventDispatchers|CreateEvent :!event Custom|AddTime)))))
      (bind _returnvalue (SaveGame|DoesSaveGameExist (Variables|Default|GetslotName)))
      (if _returnvalue
        (bind _returnvalue_2 (SaveGame|LoadGamefromSlot (Variables|Default|GetslotName)))
        (bind _asbp_high_score (Utilities|Casting|CastToBP_HighScore _returnvalue_2))
        (Variables|Default|SetHighScore (Variables|/Game/MoscowLeaders2023/Core/FileSystem/BP_HighScore.BP_HighScore_C|GethighScore _asbp_high_score))
        (else
          (bind _returnvalue_3 (SaveGame|CreateSaveGameObject "/Game/MoscowLeaders2023/Core/FileSystem/BP_HighScore.BP_HighScore_C"))
          (bind _output_get (Variables|Default|SetsubclassOfSaver _returnvalue_3))
          (Utilities|Casting|CastToBP_HighScore _output_get))))
    (:then_1
      (CallFunction|StartCountdown))))

(fn ConstructionScript)

(fn AddTimetoTimer
  (params (TimeToAdd :type Float%20%28double-precision%29))
  (bind _returnvalue (Utilities|Time|SetTimerbyEvent (EventDispatchers|CreateEvent :!event Custom|LoseOutOfTime) (+ (Utilities|Time|GetTimerRemainingTimebyHandle (Variables|Default|GetCurrentTime)) TimeToAdd)))
  (Variables|Default|SetCurrentTime _returnvalue)
  (return))